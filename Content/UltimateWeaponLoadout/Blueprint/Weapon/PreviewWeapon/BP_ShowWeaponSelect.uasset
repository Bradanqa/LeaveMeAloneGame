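; Preview stage actor for the weapon loadout menu, showing the selected weapon or the character holding the current one.
; It respawns a BP_Weaponbase per selection, switches between weapon and character cameras, and opens the customization widget in modify mode.
; Mouse drag rotates the preview with interpolation, while timelines move the weapon camera between positions.
; Wheel input sets a target FOV, but the per-frame zoom and centering calls are disconnected.
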(event Custom|TimeNewPositionCamera
  (params (InTransform :type Transform%20%28by%20ref%29))
  ;[1 1 1] Animation Move Camera
  (Variables|Default|SetCanRotate false)
  (CallFunction|ResetWeaponRotation)
  (Components|Timeline|SetPlayRate (Variables|Default|GetNewPositionCamera) 2.0)
  (bind _alpha (Timeline|NewPositionCamera PlayFromStart)
    (:Update
      (Transformation|SetRelativeLocationAndRotation (Variables|Default|GetCameraWeapon) (.Location (Math|Transform|BreakTransform (Math|Transform|Lerp(Transform) (Variables|Default|GetCurrentPositionCamera) InTransform _alpha))) (.Rotation (Math|Transform|BreakTransform (Math|Transform|Lerp(Transform) (Variables|Default|GetCurrentPositionCamera) InTransform _alpha))) false false))))

(event Custom|TimeResetPositionCamera
  ;[1 1 1] Animation Move Camera
  (Components|Timeline|SetPlayRate (Variables|Default|GetResetPositionCamera) 2.0)
  (bind _alpha (Timeline|ResetPositionCamera PlayFromStart)
    (:Update
      (Transformation|SetRelativeLocationAndRotation (Variables|Default|GetCameraWeapon) (.Location (Math|Transform|BreakTransform (Math|Transform|Lerp(Transform) (Transformation|GetRelativeTransform (Variables|Default|GetCameraWeapon)) (Math|Transform|MakeTransform "0, 0, 0" "0, 0, 0" "1.000000,1.000000,1.000000") _alpha))) (.Rotation (Math|Transform|BreakTransform (Math|Transform|Lerp(Transform) (Transformation|GetRelativeTransform (Variables|Default|GetCameraWeapon)) (Math|Transform|MakeTransform "0, 0, 0" "0, 0, 0" "1.000000,1.000000,1.000000") _alpha))) false false))
    (:Finished
      (Variables|Default|SetCanRotate true))))

(event Custom|ResetWeaponRotation
  ;[1 1 1] Animation Move Camera
  (bind _weapon_current_show (Variables|Default|GetWeapon%20Current%20Show)
    (:then
      (Transformation|SetRelativeRotation (Variables|/Game/UltimateWeaponLoadout/Blueprint/Weapon/BP_Weaponbase.BP_Weaponbase_C|GetSkeletalMesh _weapon_current_show) (Variables|Default|GetRelative%20Rotation%20Orirgin) false false)
      (Variables|Default|SetTargetRotate "0, 0, 0"))
    (:else)))

(event Custom|BeginModifyWeapon
  (params (S%20Weapon%20Config :type S%20Weapon%20Config%20Structure) (WBMain%20Select%20Weapon :type WB%20Main%20Select%20Weapon%20Object%20Reference))
  (bind _sceneweapon (Variables|Default|GetSceneWeapon))
  ;[1 1 1] Config Weapon
  (Variables|Default|SetS%20Weapon%20Config S%20Weapon%20Config)
  (Variables|Default|SetWBMain%20Select%20Weapon WBMain%20Select%20Weapon)
  (Variables|/Script/Engine.SpringArmComponent|SetTargetArmLength (Variables|Default|GetSpringArmWeapon) (Variables|Default|GetTargetArm))
  (bind _output_get (Variables|Default|SetTargetFOV (select (Variables|Default|GetCanZoom) (Math|Float|Clamp(Float) (Variables|Default|GetInitialFOV) (Variables|Default|GetMinFOV) (Variables|Default|GetMaxFOV)) (Variables|Default|GetInitialFOV))))
  (Camera|SetFieldOfView (Variables|Default|GetCameraWeapon) _output_get)
  (Variables|Default|SetBaseRelativeLocation (Variables|/Script/Engine.SceneComponent|GetRelativeLocation _sceneweapon))
  (Variables|Default|SetRelative%20Rotation%20Orirgin (Variables|/Script/Engine.SceneComponent|GetRelativeRotation _sceneweapon))
  (bind _weapon_current_show (Variables|Default|GetWeapon%20Current%20Show)
    (:then
      (Actor|DestroyActor _weapon_current_show))
    (:else
      _))
  (bind _returnvalue (Game|SpawnActorfromClass "/Game/UltimateWeaponLoadout/Blueprint/Weapon/BP_Weaponbase.BP_Weaponbase_C" (Transformation|GetWorldTransform (Variables|Default|GetSceneWeapon)) "Undefined" "OverrideRootScale" 0 (Variables|Default|GetS%20Weapon%20Config) "None" 0))
  (Variables|Default|SetWeapon%20Current%20Show _returnvalue)
  (bind _returnvalue_2 (UserInterface|CreateWidget "/Game/UltimateWeaponLoadout/Blueprint/Widget/Mode1/WB_CustomizationMode1.WB_CustomizationMode1_C" (Variables|Default|GetOwning%20Player%20Controller) (Variables|Default|GetWeapon%20Current%20Show) (Variables|Default|GetWBMain%20Select%20Weapon) (Variables|Default|GetS%20Weapon%20Config)))
  (UserInterface|Viewport|AddtoViewport _returnvalue_2 0))

(event Custom|SelectWeapon
  (params (S_WeaponConfig :type S%20Weapon%20Config%20Structure))
  ;[1 1 1] New Weapon Visible
  (bind _weapon_current_show (Variables|Default|GetWeapon%20Current%20Show)
    (:then
      (Actor|DestroyActor _weapon_current_show))
    (:else
      _))
  (bind _returnvalue (Game|SpawnActorfromClass "/Game/UltimateWeaponLoadout/Blueprint/Weapon/BP_Weaponbase.BP_Weaponbase_C" (Transformation|GetWorldTransform (Variables|Default|GetSceneWeapon)) "Undefined" "OverrideRootScale" 0 S_WeaponConfig "None" 0))
  (Variables|Default|SetWeapon%20Current%20Show _returnvalue)
  (CallFunction|SetNewLocationCamera (Variables|Default|GetCameraLocationSelectWeapon))
  (Components|Activation|SetActive (Variables|Default|GetCameraCharacter) false false)
  (Components|Activation|SetActive (Variables|Default|GetCameraWeapon) true false)
  (Variables|Default|SetCharacterActive? false))

(event Custom|ActiveCameraCharacter
  ;[1 1 1] Refresh Character
  (Variables|Default|SetTargetRotate "0.000000,0.000000,-100.000000")
  (Components|Activation|SetActive (Variables|Default|GetCameraCharacter) true false)
  (Components|Activation|SetActive (Variables|Default|GetCameraWeapon) false false)
  (CallFunction|RefreshCharacter)
  (Variables|Default|SetCanRotate true)
  (Variables|Default|SetCharacterActive? true))

(event Custom|RefreshCharacter
  ;[1 1 1] Refresh Character
  (bind _character (Variables|Default|GetCharacter)
    (:then
      (bind _mesh (Variables|/Script/Engine.Character|GetMesh _character)
        (:then
          (Components|SkeletalMesh|SetSkeletalMeshAsset (Variables|Default|GetSkeletalMesh) (Variables|/Script/Engine.SkeletalMeshComponent|GetSkeletalMeshAsset _mesh))
          (bind _weapon_current (Variables|/Game/UltimateWeaponLoadout/Blueprint/BP_ComponentUltimateWeaponLoadout.BP_ComponentUltimateWeaponLoadout_C|GetWeapon%20Current (Variables|Default|GetComponent))
            (:then
              (Components|Animation|SetAnimationMode (Variables|Default|GetSkeletalMesh) "AnimationSingleNode" true)
              (Components|Animation|SetAnimation (Variables|Default|GetSkeletalMesh) (.AnimationShowCaseWeapon (Utilities|Struct|BreakS_WeaponConfig (Variables|/Game/UltimateWeaponLoadout/Blueprint/Weapon/BP_Weaponbase.BP_Weaponbase_C|GetS_WeaponConfig _weapon_current))))
              (Audio|Components|Audio|Play (Variables|Default|GetSkeletalMesh) true))
            (:else
              (Components|Animation|SetAnimationMode (Variables|Default|GetSkeletalMesh) "AnimationBlueprint" true)
              (bind _animclass (Variables|/Script/Engine.SkeletalMeshComponent|GetAnimClass _mesh)
                (:then
                  (Class|SkeletalMeshComponent|SetAnimClass (Variables|Default|GetSkeletalMesh) _animclass))
                (:else))))
          (bind _weapon_current_show (Variables|Default|GetWeapon%20Current%20Show)
            (:then
              (Actor|DestroyActor _weapon_current_show))
            (:else
              _))
          (bind _returnvalue (Game|SpawnActorfromClass "/Game/UltimateWeaponLoadout/Blueprint/Weapon/BP_Weaponbase.BP_Weaponbase_C" (Transformation|GetWorldTransform (Variables|Default|GetSceneWeapon)) "Undefined" "OverrideRootScale" 0 (Variables|/Game/UltimateWeaponLoadout/Blueprint/Weapon/BP_Weaponbase.BP_Weaponbase_C|GetS_WeaponConfig _weapon_current) "None" 0))
          (Variables|Default|SetWeapon%20Current%20Show _returnvalue)
          (Transformation|AttachComponentToComponent _returnvalue (Variables|Default|GetSkeletalMesh) (Utilities|Struct|BreakS_WeaponConfig (Variables|/Game/UltimateWeaponLoadout/Blueprint/Weapon/BP_Weaponbase.BP_Weaponbase_C|GetS_WeaponConfig _weapon_current)) "SnapToTarget" "SnapToTarget" "SnapToTarget" true))
        (:else)))
    (:else)))

(event EventBeginPlay
  ;[1 1 1] Begin play
  (Variables|Default|SetOwning%20Player%20Controller (Variables|/Game/UltimateWeaponLoadout/Blueprint/BP_ComponentUltimateWeaponLoadout.BP_ComponentUltimateWeaponLoadout_C|GetOwning%20Player%20Controller (Variables|Default|GetComponent)))
  (if (Variables|Default|GetModifyWeapon?)
    (CallFunction|BeginModifyWeapon)
    (else
      (Input|EnableInput (Variables|Default|GetOwning%20Player%20Controller))
      (Variables|/Script/Engine.PlayerController|SetbShowMouseCursor (Variables|Default|GetOwning%20Player%20Controller) true)
      (Input|SetInputModeGameandUI (Variables|Default|GetOwning%20Player%20Controller) 0 "DoNotLock" true false))))

(event EventDestroyed
  ;[1 1 1] Event Destroyer Actor
  (bind _component (Variables|Default|GetComponent)
    (:then
      (Default|RemoveMainLoadout _component)
      (bind _weapon_current_show (Variables|Default|GetWeapon%20Current%20Show)
        (:then
          (Actor|DestroyActor _weapon_current_show))
        (:else)))
    (:else)))

(event EventTick
  (params (DeltaSeconds :type Float%20%28single-precision%29))
  ;[1 1 1] Event Tick
  (if (or (Variables|Default|GetModifyWeapon?) (Variables|Default|GetCharacterActive?))
    (CallFunction|GetPlayerInputStrength)
    (CallFunction|RotateWeapon)))

(event Input|MouseEvents|MouseWheelAxis
  (params (AxisValue :type Float%20%28single-precision%29))
  ;[1 1 1] Move Weapon
  (CallFunction|SetFOV AxisValue))

(event Input|MouseEvents|LeftMouseButton
  (params (Key :type Key%20Structure))
  (bind _owning_player_controller (Variables|Default|GetOwning%20Player%20Controller))
  ;[1 1 1] Move Weapon
  (:Pressed
    (Variables|Default|SetInteracting true)
    (Variables|/Script/Engine.PlayerController|SetbShowMouseCursor _owning_player_controller false))
  (:Released
    (Variables|Default|SetInteracting false)
    (Variables|/Script/Engine.PlayerController|SetbShowMouseCursor _owning_player_controller true)))

(fn ConstructionScript)

(fn SetFOV
  (params (Axis :type Float%20%28double-precision%29))
  (Variables|Default|SetTargetFOV (Math|Float|Clamp(Float) (+ (* Axis (Variables|Default|GetWheelAxisMultiply) -1.0) (Variables|Default|GetTargetFOV)) (Variables|Default|GetMinFOV) (Variables|Default|GetMaxFOV))))

(fn GetPlayerInputStrength
  (bind _owning_player_controller (Variables|Default|GetOwning%20Player%20Controller))
  (bind (_deltax _deltay) (Class|PlayerController|GetInputMouseDelta _owning_player_controller))
  (if (Variables|Default|GetInteracting)
    (Variables|Default|SetTargetRotate (Math|Rotator|MakeRotator (+ (* _deltax -1.0 (Variables|Default|GetRotationSpeed)) (.Roll (Math|Rotator|BreakRotator (Variables|Default|GetTargetRotate)))) (+ (.Pitch (Math|Rotator|BreakRotator (Variables|Default|GetTargetRotate))) (* _deltay (Variables|Default|GetRotationSpeed) -1.0 -1.0)) 0.0))))

(fn RotateWeapon
  (bind _targetrotate (Variables|Default|GetTargetRotate))
  (bind (_roll _pitch) (Math|Rotator|BreakRotator _targetrotate))
  (Variables|Default|GetWeapon%20Current%20Show
    (:then
      (if (Variables|Default|GetCanRotate)
        (if (Variables|Default|GetCharacterActive?)
          (Transformation|SetRelativeRotation (Variables|Default|GetSkeletalMesh) (Math|Interpolation|RInterpTo (Variables|/Script/Engine.SceneComponent|GetRelativeRotation (Variables|Default|GetSkeletalMesh)) (Math|Rotator|MakeRotator 0.0 0.0 (.Roll (Math|Rotator|BreakRotator (Variables|Default|GetTargetRotate)))) (Utilities|Time|GetWorldDeltaSeconds) (Variables|Default|GetRotationInterp)) false false)
          (else
            (Transformation|SetRelativeRotation (Variables|/Game/UltimateWeaponLoadout/Blueprint/Weapon/BP_Weaponbase.BP_Weaponbase_C|GetSkeletalMesh (Variables|Default|GetWeapon%20Current%20Show)) (Math|Interpolation|RInterpTo (Variables|/Script/Engine.SceneComponent|GetRelativeRotation (Variables|/Game/UltimateWeaponLoadout/Blueprint/Weapon/BP_Weaponbase.BP_Weaponbase_C|GetSkeletalMesh (Variables|Default|GetWeapon%20Current%20Show))) (Math|Rotator|MakeRotator 0.0 (Math|Float|Clamp(Float) _pitch -4e+01 4e+01) _roll) (Utilities|Time|GetWorldDeltaSeconds) (Variables|Default|GetRotationInterp)) false false)))))
    (:else)))

(fn SetCameraOffset
  (if (Variables|Default|GetCenterWeapon)
    (Variables|/Script/Engine.SpringArmComponent|SetSocketOffset (Variables|Default|GetSpringArmWeapon) (Math|Interpolation|VInterpTo (Variables|/Script/Engine.SpringArmComponent|GetSocketOffset (Variables|Default|GetSpringArmWeapon)) "0, 0, 0" (Utilities|Time|GetWorldDeltaSeconds) (Variables|Default|GetCenterSpeed)))))

(fn ChangeFOV
  (if (Variables|Default|GetCanZoom)
    (Camera|SetFieldOfView (Variables|Default|GetCameraWeapon) (Math|Interpolation|FInterpTo (Variables|/Script/Engine.CameraComponent|GetFieldOfView (Variables|Default|GetCameraWeapon)) (Variables|Default|GetTargetFOV) (Utilities|Time|GetWorldDeltaSeconds) (Variables|Default|GetZoomInterpSpeed)))))

(fn SetNewLocationCamera
  (params (New%20Transform :type Transform))
  (Variables|Default|SetCurrentPositionCamera (Transformation|GetRelativeTransform (Variables|Default|GetCameraWeapon)))
  (CallFunction|TimeNewPositionCamera New%20Transform))

(fn ResetCameraLocation
  (CallFunction|TimeResetPositionCamera))